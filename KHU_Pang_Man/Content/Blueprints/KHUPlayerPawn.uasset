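; KHUPlayerPawn is the player-controlled Blueprint, handling walking and looking around through input events.
; Move axes add movement input along the Camera's forward and right vectors, while look axes feed controller pitch and yaw.
; Shift is commented as a speed boost, but press and release both set CharacterMovement's max walk speed to the same value, so the handler never produces a faster speed.
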(event `InputAxis|LookUpDown`
  (params (AxisValue :type "Float (single-precision)"))
  (`self.AddControllerPitchInput` AxisValue))

(event `InputAxis|MoveForBack`
  (params (AxisValue :type "Float (single-precision)"))
  (`self.AddMovementInput` (`SceneComponent.GetForwardVector` (`self.Camera`)) AxisValue) ; 앞뒤로 이동
)

(event `InputAxis|LookRightLeft`
  (params (AxisValue :type "Float (single-precision)"))
  (`self.AddControllerYawInput` AxisValue))

(event `InputAxis|MoveRightLeft`
  (params (AxisValue :type "Float (single-precision)"))
  (`self.AddMovementInput` (`SceneComponent.GetRightVector` (`self.Camera`)) AxisValue) ; 좌우로 이동
)

(event `InputAction|Shift`
  (params (Key :type "Key Structure"))
  (bind _charactermovement (`self.CharacterMovement`))
  (:`Pressed`
    (set `CharacterMovementComponent.MaxWalkSpeed` 200.0 _charactermovement) ; 키를 누르면 속도 증가
  )
  (:`Released`
    (set `CharacterMovementComponent.MaxWalkSpeed` 200.0 _charactermovement) ; 키를 때면 속도 복귀
  ))

(fn `UserConstructionScript`)